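; Player character Blueprint that changes the color saturation of its camera view when it receives a color power.
; GetColorPower adds the incoming color to an accumulated TargetColor and restarts the HealColor timeline.
; Each timeline update lerps the camera's current post-process saturation RGB toward that target, clamps the vector's length to 1 and keeps W unchanged.
; BeginPlay, overlap and Tick are unused.
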(event Custom|GetColorPower
  (params (GetColor :type Vector))
  (bind _camera (Variables|Default|GetCamera))
  (Variables|Default|SetTargetColor (+ (Variables|Default|GetTargetColor) GetColor))
  (bind _alpha (Timeline|Timeline_HealColor PlayFromStart)
    (:Update
      (Variables|/Script/Engine.CameraComponent|SetPostProcessSettings _camera (Utilities|Struct|MakePostProcessSettings (Math|Vector4|MakeVector4 (.x (Math|Vector|ClampVectorSize (Math|Vector|MakeVector (.x (Math|Vector|Lerp(Vector) (Math|Vector|MakeVector (.x (Utilities|Struct|BreakPostProcessSettings (Variables|/Script/Engine.CameraComponent|GetPostProcessSettings _camera))) (.y (Utilities|Struct|BreakPostProcessSettings (Variables|/Script/Engine.CameraComponent|GetPostProcessSettings _camera))) (.z (Utilities|Struct|BreakPostProcessSettings (Variables|/Script/Engine.CameraComponent|GetPostProcessSettings _camera)))) (Math|Vector|MakeVector (.x (Variables|Default|GetTargetColor)) (.y (Variables|Default|GetTargetColor)) (.z (Variables|Default|GetTargetColor))) _alpha)) (.y (Math|Vector|Lerp(Vector) (Math|Vector|MakeVector (.x (Utilities|Struct|BreakPostProcessSettings (Variables|/Script/Engine.CameraComponent|GetPostProcessSettings _camera))) (.y (Utilities|Struct|BreakPostProcessSettings (Variables|/Script/Engine.CameraComponent|GetPostProcessSettings _camera))) (.z (Utilities|Struct|BreakPostProcessSettings (Variables|/Script/Engine.CameraComponent|GetPostProcessSettings _camera)))) (Math|Vector|MakeVector (.x (Variables|Default|GetTargetColor)) (.y (Variables|Default|GetTargetColor)) (.z (Variables|Default|GetTargetColor))) _alpha)) (.z (Math|Vector|Lerp(Vector) (Math|Vector|MakeVector (.x (Utilities|Struct|BreakPostProcessSettings (Variables|/Script/Engine.CameraComponent|GetPostProcessSettings _camera))) (.y (Utilities|Struct|BreakPostProcessSettings (Variables|/Script/Engine.CameraComponent|GetPostProcessSettings _camera))) (.z (Utilities|Struct|BreakPostProcessSettings (Variables|/Script/Engine.CameraComponent|GetPostProcessSettings _camera)))) (Math|Vector|MakeVector (.x (Variables|Default|GetTargetColor)) (.y (Variables|Default|GetTargetColor)) (.z (Variables|Default|GetTargetColor))) _alpha))) 0.0 1.0)) (.y (Math|Vector|ClampVectorSize (Math|Vector|MakeVector (.x (Math|Vector|Lerp(Vector) (Math|Vector|MakeVector (.x (Utilities|Struct|BreakPostProcessSettings (Variables|/Script/Engine.CameraComponent|GetPostProcessSettings _camera))) (.y (Utilities|Struct|BreakPostProcessSettings (Variables|/Script/Engine.CameraComponent|GetPostProcessSettings _camera))) (.z (Utilities|Struct|BreakPostProcessSettings (Variables|/Script/Engine.CameraComponent|GetPostProcessSettings _camera)))) (Math|Vector|MakeVector (.x (Variables|Default|GetTargetColor)) (.y (Variables|Default|GetTargetColor)) (.z (Variables|Default|GetTargetColor))) _alpha)) (.y (Math|Vector|Lerp(Vector) (Math|Vector|MakeVector (.x (Utilities|Struct|BreakPostProcessSettings (Variables|/Script/Engine.CameraComponent|GetPostProcessSettings _camera))) (.y (Utilities|Struct|BreakPostProcessSettings (Variables|/Script/Engine.CameraComponent|GetPostProcessSettings _camera))) (.z (Utilities|Struct|BreakPostProcessSettings (Variables|/Script/Engine.CameraComponent|GetPostProcessSettings _camera)))) (Math|Vector|MakeVector (.x (Variables|Default|GetTargetColor)) (.y (Variables|Default|GetTargetColor)) (.z (Variables|Default|GetTargetColor))) _alpha)) (.z (Math|Vector|Lerp(Vector) (Math|Vector|MakeVector (.x (Utilities|Struct|BreakPostProcessSettings (Variables|/Script/Engine.CameraComponent|GetPostProcessSettings _camera))) (.y (Utilities|Struct|BreakPostProcessSettings (Variables|/Script/Engine.CameraComponent|GetPostProcessSettings _camera))) (.z (Utilities|Struct|BreakPostProcessSettings (Variables|/Script/Engine.CameraComponent|GetPostProcessSettings _camera)))) (Math|Vector|MakeVector (.x (Variables|Default|GetTargetColor)) (.y (Variables|Default|GetTargetColor)) (.z (Variables|Default|GetTargetColor))) _alpha))) 0.0 1.0)) (.z (Math|Vector|ClampVectorSize (Math|Vector|MakeVector (.x (Math|Vector|Lerp(Vector) (Math|Vector|MakeVector (.x (Utilities|Struct|BreakPostProcessSettings (Variables|/Script/Engine.CameraComponent|GetPostProcessSettings _camera))) (.y (Utilities|Struct|BreakPostProcessSettings (Variables|/Script/Engine.CameraComponent|GetPostProcessSettings _camera))) (.z (Utilities|Struct|BreakPostProcessSettings (Variables|/Script/Engine.CameraComponent|GetPostProcessSettings _camera)))) (Math|Vector|MakeVector (.x (Variables|Default|GetTargetColor)) (.y (Variables|Default|GetTargetColor)) (.z (Variables|Default|GetTargetColor))) _alpha)) (.y (Math|Vector|Lerp(Vector) (Math|Vector|MakeVector (.x (Utilities|Struct|BreakPostProcessSettings (Variables|/Script/Engine.CameraComponent|GetPostProcessSettings _camera))) (.y (Utilities|Struct|BreakPostProcessSettings (Variables|/Script/Engine.CameraComponent|GetPostProcessSettings _camera))) (.z (Utilities|Struct|BreakPostProcessSettings (Variables|/Script/Engine.CameraComponent|GetPostProcessSettings _camera)))) (Math|Vector|MakeVector (.x (Variables|Default|GetTargetColor)) (.y (Variables|Default|GetTargetColor)) (.z (Variables|Default|GetTargetColor))) _alpha)) (.z (Math|Vector|Lerp(Vector) (Math|Vector|MakeVector (.x (Utilities|Struct|BreakPostProcessSettings (Variables|/Script/Engine.CameraComponent|GetPostProcessSettings _camera))) (.y (Utilities|Struct|BreakPostProcessSettings (Variables|/Script/Engine.CameraComponent|GetPostProcessSettings _camera))) (.z (Utilities|Struct|BreakPostProcessSettings (Variables|/Script/Engine.CameraComponent|GetPostProcessSettings _camera)))) (Math|Vector|MakeVector (.x (Variables|Default|GetTargetColor)) (.y (Variables|Default|GetTargetColor)) (.z (Variables|Default|GetTargetColor))) _alpha))) 0.0 1.0)) (.w (Utilities|Struct|BreakPostProcessSettings (Variables|/Script/Engine.CameraComponent|GetPostProcessSettings _camera)))))))))

(event EventBeginPlay)

(event Collision|EventActorBeginOverlap
  (params (OtherActor :type Actor%20Object%20Reference)))

(event EventTick
  (params (DeltaSeconds :type Float%20%28single-precision%29)))

(fn ConstructionScript
  (|CallParentFunction))
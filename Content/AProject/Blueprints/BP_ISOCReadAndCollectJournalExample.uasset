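; BP_ISOCReadAndCollectJournalExample is an example Blueprint for a journal entry, by its name readable and collectible, that shows letter text on a widget component.
; On BeginPlay it calls the parent, casts the component's user widget to UI_LetterText, copies its LetterText variable into LetterContent and requests a redraw.
; The construction script only calls the parent; overlap and tick events are disabled stubs.
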(event EventBeginPlay
  (bind _widget (Variables|Default|GetWidget))
  (|CallParentFunction)
  (bind _asui_letter_text (Utilities|Casting|CastToUI_LetterText (UserInterface|GetUserWidgetObject _widget)))
  (Variables|/Game/StoryAdvTemplate/UserInterface/UI_LetterText.UI_LetterText_C|SetLetterContent _asui_letter_text (Variables|Default|GetLetterText))
  (Class|WidgetComponent|RequestRedraw _widget))

(event Collision|EventActorBeginOverlap
  (params (OtherActor :type Actor%20Object%20Reference))
  (|CallParentFunction OtherActor) ; 지금 이 노드는 비활성 상태입니다. \n핀을 끌어서 다른 노드를 연결하면 활성화됩니다.
)

(event EventTick
  (params (DeltaSeconds :type Float%20%28single-precision%29))
  (|CallParentFunction DeltaSeconds) ; 지금 이 노드는 비활성 상태입니다. \n핀을 끌어서 다른 노드를 연결하면 활성화됩니다.
)

(fn ConstructionScript
  (|CallParentFunction))
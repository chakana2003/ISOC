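; BP_ISOCCallingStorm is a use action that stages a storm event when triggered.
; UseEvent fades in wind audio, enables camera shake on the first Chameleon actor and spawns BP_ISOCStorm at a hard-coded position.
; A timeline raises and spins the storm while ramping shake strength.
; On finish, it destroys the storm, stops the shake, fades out the sound and only then calls the parent UseEvent.
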(event EventBeginPlay
  (|CallParentFunction) ; 지금 이 노드는 비활성 상태입니다. \n핀을 끌어서 다른 노드를 연결하면 활성화됩니다.
)

(event Collision|EventActorBeginOverlap
  (params (OtherActor :type Actor%20Object%20Reference))
  (|CallParentFunction OtherActor) ; 지금 이 노드는 비활성 상태입니다. \n핀을 끌어서 다른 노드를 연결하면 활성화됩니다.
)

(event EventTick
  (params (DeltaSeconds :type Float%20%28single-precision%29))
  (|CallParentFunction DeltaSeconds) ; 지금 이 노드는 비활성 상태입니다. \n핀을 끌어서 다른 노드를 연결하면 활성화됩니다.
)

(event EventUseEvent
  (bind _returnvalue (Audio|SpawnSound2D "/Game/AProject/Sound/SFX/405561__inspectorj__wind-realistic-a.405561__inspectorj__wind-realistic-a" 1.0 1.0 0.0 0))
  (Audio|Components|Audio|FadeIn _returnvalue 3.0 0.5 0.0 :!class /Script/Engine.AudioComponent)
  (bind _outactors (Actor|GetAllActorsOfClass "/Game/Chameleon/Chameleon.Chameleon_C"))
  (Variables|/Game/Chameleon/Chameleon.Chameleon_C|SetCamera%20Shake (Utilities|Array|Get(acopy) _outactors) true)
  (bind _returnvalue_2 (Game|SpawnActorfromClass "/Game/AProject/Blueprints/BP_ISOCStorm.BP_ISOCStorm_C" (Math|Transform|MakeTransform "-6308.000000,52.000000,-8500.000000" "0, 0, 0" "1,1,1") "Undefined" 0 0))
  (bind _alpha (Timeline|타임라인_0 PlayFromStart)
    (:Update
      (Transformation|SetActorLocation _returnvalue_2 (Math|Vector|Lerp(Vector) "-6308.000000,52.000000,-8500.000000" "-6308.000000,52.000000,-1110.000000" _alpha) false false)
      (Class|Actor|AddActorWorldRotation _returnvalue_2 "0,1.000000, 0")
      (Variables|/Game/Chameleon/Chameleon.Chameleon_C|SetCamera%20Shake%20Power%20%28X%29 (Utilities|Array|Get(acopy) _outactors) (Math|Float|Lerp 0.0 0.01 _alpha))
      (Variables|/Game/Chameleon/Chameleon.Chameleon_C|SetCamera%20Shake%20Power%20%28Y%29 (Utilities|Array|Get(acopy) _outactors) (Math|Float|Lerp 0.0 0.01 _alpha)))
    (:Finished
      (Actor|DestroyActor _returnvalue_2)
      (Variables|/Game/Chameleon/Chameleon.Chameleon_C|SetCamera%20Shake (Utilities|Array|Get(acopy) _outactors) false)
      (Audio|Components|Audio|FadeOut _returnvalue 1.0 0.0 :!class /Script/Engine.AudioComponent)
      (|CallParentFunction))))

(fn ConstructionScript
  (|CallParentFunction))
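; BP_MovingSun is a use-action actor that toggles the sun between two angles, animating the sky along with it.
; UseEvent finds the DirectionalLight and BP_Sky_Sphere among actors tagged "MoveSun".
; It checks the light's pitch to play a timeline forward or in reverse, lerping the rotation and refreshing the sky material each update.
; The parent UseEvent runs only when the timeline finishes.
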(event EventBeginPlay
  (|CallParentFunction) ; 지금 이 노드는 비활성 상태입니다. \n핀을 끌어서 다른 노드를 연결하면 활성화됩니다.
)

(event Collision|EventActorBeginOverlap
  (params (OtherActor :type Actor%20Object%20Reference))
  (|CallParentFunction OtherActor) ; 지금 이 노드는 비활성 상태입니다. \n핀을 끌어서 다른 노드를 연결하면 활성화됩니다.
)

(event EventTick
  (params (DeltaSeconds :type Float%20%28single-precision%29))
  (|CallParentFunction DeltaSeconds) ; 지금 이 노드는 비활성 상태입니다. \n핀을 끌어서 다른 노드를 연결하면 활성화됩니다.
)

(event EventUseEvent
  (bind _outactors (Actor|GetAllActorswithTag "MoveSun"))
  (for _array_element _outactors
    (bind _asdirectional_light (Utilities|Casting|CastToDirectionalLight _array_element)
      (:then
        (Variables|Default|SetNewVar_0 _asdirectional_light))
      (:CastFailed
        (bind _asbp_sky_sphere (Utilities|Casting|CastToBP_Sky_Sphere _array_element))
        (Variables|Default|SetNewVar_1 _asbp_sky_sphere))))
  (Utilities|IsValid (Variables|Default|GetNewVar_0)
    (:Is%20Valid
      (Utilities|IsValid (Variables|Default|GetNewVar_1)
        (:Is%20Valid
          (if (Math|Float|NearlyEqual(Float) (.pitch (Transformation|GetActorRotation (Variables|Default|GetNewVar_0))) -46.0 1.0)
            (bind _새_트랙_0 (Timeline|타임라인_0 PlayFromStart)
              (:Update
                (Transformation|SetActorRotation (Variables|Default|GetNewVar_0) (Math|Rotator|Lerp(Rotator) "-46.000000, 0, 0" "94.000000, 0, 0" _새_트랙_0))
                (Default|RefreshMaterial (Variables|Default|GetNewVar_1)))
              (:Finished
                (|CallParentFunction)))
            (else
              (Timeline|타임라인_0 ReverseFromEnd))))))))

(fn ConstructionScript
  (|CallParentFunction))
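; BP_RealEndingAction is a use action that opens the portal to the game's ending, likely the true ending.
; On UseEvent it searches all BP_PlayRoom actors for room number 10 and spawns BP_PortalToEnd just above that room's floor.
; It then shows a HUD message saying a portal was heard opening and calls the parent UseEvent.
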(event EventBeginPlay
  (|CallParentFunction) ; 지금 이 노드는 비활성 상태입니다. \n핀을 끌어서 다른 노드를 연결하면 활성화됩니다.
)

(event Collision|EventActorBeginOverlap
  (params (OtherActor :type Actor%20Object%20Reference))
  (|CallParentFunction OtherActor) ; 지금 이 노드는 비활성 상태입니다. \n핀을 끌어서 다른 노드를 연결하면 활성화됩니다.
)

(event EventTick
  (params (DeltaSeconds :type Float%20%28single-precision%29))
  (|CallParentFunction DeltaSeconds) ; 지금 이 노드는 비활성 상태입니다. \n핀을 끌어서 다른 노드를 연결하면 활성화됩니다.
)

(event EventUseEvent
  (bind _outactors (Actor|GetAllActorsOfClass "/Game/AProject/Blueprints/BP_PlayRoom.BP_PlayRoom_C"))
  (bind _array_element (Utilities|Array|ForEachLoopwithBreak _outactors :!label _label)
    (:LoopBody
      (if (== (Variables|/Game/AProject/Blueprints/BP_PlayRoom.BP_PlayRoom_C|GetRoomNum _array_element) 10)
        (Variables|Default|SetTargetRoom _array_element)
        (goto _label Break)))
    (:Completed
      (Game|SpawnActorfromClass "/Game/AProject/Blueprints/BP_PortalToEnd.BP_PortalToEnd_C" (Math|Transform|MakeTransform (+ (Transformation|GetWorldLocation (Variables|/Game/AProject/Blueprints/BP_PlayRoom.BP_PlayRoom_C|GetFloor (Variables|Default|GetTargetRoom))) "0, 0,100.000000") "0, 0, 0" "1,1,1") "Undefined" 0 0)
      (Default|DisplayHUDText (Variables|Default|GetGameController) "포털이 열리는 소리가 들렸다!")
      (|CallParentFunction))))

(fn ConstructionScript
  (|CallParentFunction))
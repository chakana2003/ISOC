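; BP_ISOCSOS is a use action that moves every actor tagged "SOS" vertically while the camera shakes.
; UseEvent plays a timeline that lerps each tagged actor's world Z between fixed heights, keeping X and Y.
; A second track drives shake power on the first Chameleon actor found in the level.
; When the timeline finishes, the shake switches off and only then does the parent UseEvent run.
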(event EventBeginPlay
  (|CallParentFunction) ; 지금 이 노드는 비활성 상태입니다. \n핀을 끌어서 다른 노드를 연결하면 활성화됩니다.
)

(event Collision|EventActorBeginOverlap
  (params (OtherActor :type Actor%20Object%20Reference))
  (|CallParentFunction OtherActor) ; 지금 이 노드는 비활성 상태입니다. \n핀을 끌어서 다른 노드를 연결하면 활성화됩니다.
)

(event EventTick
  (params (DeltaSeconds :type Float%20%28single-precision%29))
  (|CallParentFunction DeltaSeconds) ; 지금 이 노드는 비활성 상태입니다. \n핀을 끌어서 다른 노드를 연결하면 활성화됩니다.
)

(event EventUseEvent
  (bind _outactors (Actor|GetAllActorsOfClass "/Game/Chameleon/Chameleon.Chameleon_C"))
  (bind _outactors_2 (Actor|GetAllActorswithTag "SOS"))
  (Variables|/Game/Chameleon/Chameleon.Chameleon_C|SetCamera%20Shake (Utilities|Array|Get(acopy) _outactors) true)
  (bind (_direction _alpha _새_트랙_0) (Timeline|타임라인_0 PlayFromStart)
    (:Update
      (for _array_element _outactors_2
        (Transformation|SetActorLocation _array_element (Math|Vector|MakeVector (.x (Transformation|GetActorLocation _array_element)) (.y (Transformation|GetActorLocation _array_element)) (Math|Float|Lerp -1.15e+04 7.5e+03 _alpha)) false false)
        (Variables|/Game/Chameleon/Chameleon.Chameleon_C|SetCamera%20Shake%20Power%20%28X%29 (Utilities|Array|Get(acopy) _outactors) (Math|Float|Lerp 0.0 0.02 _새_트랙_0))
        (Variables|/Game/Chameleon/Chameleon.Chameleon_C|SetCamera%20Shake%20Power%20%28Y%29 (Utilities|Array|Get(acopy) _outactors) (Math|Float|Lerp 0.0 0.02 _새_트랙_0))))
    (:Finished
      (Variables|/Game/Chameleon/Chameleon.Chameleon_C|SetCamera%20Shake (Utilities|Array|Get(acopy) _outactors) false)
      (|CallParentFunction))))

(fn ConstructionScript
  (|CallParentFunction))
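; Base use-action Blueprint that, on spawn, updates an inventory item's text and shows a message to the player.
; BeginPlay overwrites the GameController inventory entry at the MenuPawn's selected index with UpdateName and UpdateDescription, copying every other field unchanged.
; It then displays ActiveMessage as HUD text, retrying on a short delay until GameController is valid.
; The inventory write runs before that validity check.
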(event EventBeginPlay
  (bind _gamecontroller (Variables|Default|GetGameController))
  (bind _menupawn (Variables|Default|GetMenuPawn))
  (bind _gamecontroller_2 (Variables|Default|GetGameController))
  (bind _inventory (Variables|/Game/StoryAdvTemplate/Blueprints/BP_GameController.BP_GameController_C|GetInventory _gamecontroller_2))
  (bind _selecteditemindex (Variables|/Game/StoryAdvTemplate/Blueprints/Core/GameMenu/BP_MenuPawn.BP_MenuPawn_C|GetSelectedItemIndex _menupawn))
  (bind _output (Utilities|Array|Get(acopy) _inventory _selecteditemindex))
  (|CallParentFunction)
  (Utilities|Array|SetArrayElem _inventory _selecteditemindex (Utilities|Struct|MakeBP_InventoryItem (Variables|UpdateItemName|GetUpdateName) (Variables|UpdateItemName|GetUpdateDescription) (.additionaldescription _output) (.objectimage _output) (.objectmesh _output) (.discardable? _output) (.iskey? _output) (.keyid _output) (.useaction _output) (.discardwhenused? _output) (.inspectdistance _output) (.objectscale _output) (.lettertype _output) (.simpleletter _output) (.uifontletter _output) (.containsclue _output)))
  (Utilities|IsValid _gamecontroller :!label _label
    (:Is%20Valid
      (Default|DisplayHUDText _gamecontroller (Variables|UpdateItemName|GetActiveMessage)))
    (:Is%20Not%20Valid
      (Utilities|FlowControl|Delay 0.2)
      (goto _label))))

(event Collision|EventActorBeginOverlap
  (params (OtherActor :type Actor%20Object%20Reference))
  (|CallParentFunction OtherActor) ; 지금 이 노드는 비활성 상태입니다. \n핀을 끌어서 다른 노드를 연결하면 활성화됩니다.
)

(event EventTick
  (params (DeltaSeconds :type Float%20%28single-precision%29))
  (|CallParentFunction DeltaSeconds) ; 지금 이 노드는 비활성 상태입니다. \n핀을 끌어서 다른 노드를 연결하면 활성화됩니다.
)

(fn ConstructionScript
  (|CallParentFunction))

(fn NewFunction0)
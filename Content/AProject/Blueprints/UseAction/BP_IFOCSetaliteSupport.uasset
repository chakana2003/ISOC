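; BP_IFOCSetaliteSupport is a use-action Blueprint for satellite support that presents a search for nearby creatures.
; UseEvent plays a machine sound, then steps through timed Korean HUD messages with animated dots via the GameController.
; It performs no detection: it always replays the sound, reports that no creatures were found and it is deactivating, then calls the parent UseEvent.
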(event EventBeginPlay
  (|CallParentFunction) ; 지금 이 노드는 비활성 상태입니다. \n핀을 끌어서 다른 노드를 연결하면 활성화됩니다.
)

(event Collision|EventActorBeginOverlap
  (params (OtherActor :type Actor%20Object%20Reference))
  (|CallParentFunction OtherActor) ; 지금 이 노드는 비활성 상태입니다. \n핀을 끌어서 다른 노드를 연결하면 활성화됩니다.
)

(event EventTick
  (params (DeltaSeconds :type Float%20%28single-precision%29))
  (|CallParentFunction DeltaSeconds) ; 지금 이 노드는 비활성 상태입니다. \n핀을 끌어서 다른 노드를 연결하면 활성화됩니다.
)

(event EventUseEvent
  (Audio|SpawnSound2D "/Game/AProject/Sound/SFX/machine01_Cue.machine01_Cue" 1.0 1.0 0.0 0)
  (Utilities|FlowControl|Delay 1.0)
  (Default|DisplayHUDText (Variables|Default|GetGameController) "주변의 생물체를 찾고있습니다.")
  (Utilities|FlowControl|Delay 3.0)
  (Default|DisplayHUDText (Variables|Default|GetGameController) ".")
  (Utilities|FlowControl|Delay 0.5)
  (Default|DisplayHUDText (Variables|Default|GetGameController) "..")
  (Utilities|FlowControl|Delay 0.5)
  (Default|DisplayHUDText (Variables|Default|GetGameController) "...")
  (Utilities|FlowControl|Delay 0.5)
  (Default|DisplayHUDText (Variables|Default|GetGameController) ".")
  (Utilities|FlowControl|Delay 0.5)
  (Default|DisplayHUDText (Variables|Default|GetGameController) "..")
  (Audio|SpawnSound2D "/Game/AProject/Sound/SFX/machine01_Cue.machine01_Cue" 1.0 1.0 0.0 0)
  (Default|DisplayHUDText (Variables|Default|GetGameController) "주변에 발견된 생물체가 없음으로 비활성화됩니다.")
  (|CallParentFunction))

(fn ConstructionScript
  (|CallParentFunction))
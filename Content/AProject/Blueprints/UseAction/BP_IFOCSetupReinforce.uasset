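; Use-action Blueprint that temporarily raises reinforcement walls, the actors tagged "ReinForce".
; UseEvent plays a machine sound and runs a timeline that lerps each tagged actor's Z from underground depth upward, keeping X and Y.
; After a delay it shows a Korean HUD deactivation message, replays the sound and reverses the timeline to lower them.
; The parent UseEvent runs only after that reverse pass and another delay.
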(event EventBeginPlay
  (|CallParentFunction) ; 지금 이 노드는 비활성 상태입니다. \n핀을 끌어서 다른 노드를 연결하면 활성화됩니다.
)

(event Collision|EventActorBeginOverlap
  (params (OtherActor :type Actor%20Object%20Reference))
  (|CallParentFunction OtherActor) ; 지금 이 노드는 비활성 상태입니다. \n핀을 끌어서 다른 노드를 연결하면 활성화됩니다.
)

(event EventTick
  (params (DeltaSeconds :type Float%20%28single-precision%29))
  (|CallParentFunction DeltaSeconds) ; 지금 이 노드는 비활성 상태입니다. \n핀을 끌어서 다른 노드를 연결하면 활성화됩니다.
)

(event EventUseEvent
  (Audio|PlaySound2D "/Game/AProject/Sound/SFX/machine01_Cue.machine01_Cue" 1.0 1.0 0.0 0 0)
  (bind _outactors (Actor|GetAllActorswithTag "ReinForce"))
  (bind (_direction _alpha) (Timeline|타임라인_0 PlayFromStart)
    (:Update
      (for _array_element _outactors
        (Transformation|SetActorLocation _array_element (Math|Vector|MakeVector (.x (Transformation|GetActorLocation _array_element)) (.y (Transformation|GetActorLocation _array_element)) (Math|Float|Lerp -3e+03 -1e+03 _alpha)) false false)))
    (:Finished
      (Utilities|FlowControl|Delay 1e+01)
      (switch Utilities|FlowControl|Switch|SwitchonETimelineDirection _direction
        (:Forward
          (Default|DisplayHUDText (Variables|Default|GetGameController) "강화벽 비 활성화.")
          (Audio|PlaySound2D "/Game/AProject/Sound/SFX/machine01_Cue.machine01_Cue" 1.0 1.0 0.0 0 0)
          (Timeline|타임라인_0 ReverseFromEnd))
        (:Backward
          (|CallParentFunction))))))

(fn ConstructionScript
  (|CallParentFunction))
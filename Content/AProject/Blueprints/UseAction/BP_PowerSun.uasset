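; BP_PowerSun is a use-action Blueprint that boosts the sun's brightness when used.
; UseEvent fades in a looping heat sound and plays a timeline that lerps the intensity of the first DirectionalLight found in the level from a normal to a very bright level.
; When the timeline finishes, it fades the sound out and then calls the parent UseEvent.
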(event EventBeginPlay
  (|CallParentFunction) ; 지금 이 노드는 비활성 상태입니다. \n핀을 끌어서 다른 노드를 연결하면 활성화됩니다.
)

(event Collision|EventActorBeginOverlap
  (params (OtherActor :type Actor%20Object%20Reference))
  (|CallParentFunction OtherActor) ; 지금 이 노드는 비활성 상태입니다. \n핀을 끌어서 다른 노드를 연결하면 활성화됩니다.
)

(event EventTick
  (params (DeltaSeconds :type Float%20%28single-precision%29))
  (|CallParentFunction DeltaSeconds) ; 지금 이 노드는 비활성 상태입니다. \n핀을 끌어서 다른 노드를 연결하면 활성화됩니다.
)

(event EventUseEvent
  (bind _returnvalue (Audio|SpawnSound2D "/Game/AProject/Sound/SFX/195508__cubicapocalypse__heat-loop1_Cue.195508__cubicapocalypse__heat-loop1_Cue" 1.0 1.0 0.0 0))
  (Audio|Components|Audio|FadeIn _returnvalue 3.0 1.0 0.0 :!class /Script/Engine.AudioComponent)
  (bind _outactors (Actor|GetAllActorsOfClass "/Script/Engine.DirectionalLight"))
  (bind _새_트랙_0 (Timeline|타임라인_0 PlayFromStart)
    (:Update
      (Rendering|Components|Light|SetIntensity (Variables|/Script/Engine.Light|GetLightComponent (Utilities|Array|Get(acopy) _outactors)) (Math|Float|Lerp 1e+01 5e+02 _새_트랙_0)))
    (:Finished
      (Audio|Components|Audio|FadeOut _returnvalue 1.0 0.0 :!class /Script/Engine.AudioComponent)
      (|CallParentFunction))))

(fn ConstructionScript
  (|CallParentFunction))
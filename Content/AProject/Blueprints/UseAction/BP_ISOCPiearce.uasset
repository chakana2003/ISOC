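; Inventory item use action that temporarily moves spike actors tagged "DA", with machine sounds.
; A timeline slides them along their negative up vectors, waits, shows a "spikes deactivated" HUD message, then reverses.
; BeginPlay rewrites the selected inventory slot without its use action, blocking reuse during the cycle.
; After the reverse and another delay, it restores this class on the item cached from slot 0, then calls parent UseEvent.
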(event EventBeginPlay
  (bind _menupawn (Variables|Default|GetMenuPawn))
  (bind _gamecontroller (Variables|Default|GetGameController))
  (bind _inventory (Variables|/Game/StoryAdvTemplate/Blueprints/BP_GameController.BP_GameController_C|GetInventory _gamecontroller))
  (bind _selecteditemindex (Variables|/Game/StoryAdvTemplate/Blueprints/Core/GameMenu/BP_MenuPawn.BP_MenuPawn_C|GetSelectedItemIndex _menupawn))
  (bind _output (Utilities|Array|Get(acopy) _inventory _selecteditemindex))
  (|CallParentFunction)
  (Utilities|Array|SetArrayElem _inventory _selecteditemindex (Utilities|Struct|MakeBP_InventoryItem (.objectname _output) (.objectdescription _output) (.additionaldescription _output) (.objectimage _output) (.objectmesh _output) (.discardable? _output) (.iskey? _output) (.keyid _output) 0 (.discardwhenused? _output) (.inspectdistance _output) (.objectscale _output) (.lettertype _output) (.simpleletter _output) (.uifontletter _output) (.containsclue _output)))
  (Variables|Default|SetNewVar_2 (Utilities|Array|Get(acopy) _inventory)))

(event Collision|EventActorBeginOverlap
  (params (OtherActor :type Actor%20Object%20Reference))
  (|CallParentFunction OtherActor) ; 지금 이 노드는 비활성 상태입니다. \n핀을 끌어서 다른 노드를 연결하면 활성화됩니다.
)

(event EventTick
  (params (DeltaSeconds :type Float%20%28single-precision%29))
  (|CallParentFunction DeltaSeconds) ; 지금 이 노드는 비활성 상태입니다. \n핀을 끌어서 다른 노드를 연결하면 활성화됩니다.
)

(event EventUseEvent
  (bind _newvar_2 (Variables|Default|GetNewVar_2))
  (bind _gamecontroller (Variables|Default|GetGameController))
  (bind _inventory (Variables|/Game/StoryAdvTemplate/Blueprints/BP_GameController.BP_GameController_C|GetInventory _gamecontroller))
  (bind _returnvalue (Utilities|Array|FindItem _inventory _newvar_2))
  (bind _output (Utilities|Array|Get(acopy) _inventory _returnvalue))
  (Audio|PlaySound2D "/Game/AProject/Sound/SFX/machine01_Cue.machine01_Cue" 1.0 1.0 0.0 0 0)
  (bind _outactors (Actor|GetAllActorswithTag "DA"))
  (bind _output_get (Variables|Default|SetNewVar_1 _outactors))
  (for _array_element _output_get
    (Utilities|Array|Add (Variables|Default|GetNewVar_0_0) (Transformation|GetActorLocation _array_element)))
  (bind (_direction _alpha) (Timeline|타임라인_1 PlayFromStart)
    (:Update
      (for (_array_element_2 _array_index) _output_get
        (Transformation|SetActorLocation _array_element_2 (Math|Vector|Lerp(Vector) (Utilities|Array|Get(acopy) (Variables|Default|GetNewVar_0_0) _array_index) (+ (Utilities|Array|Get(acopy) (Variables|Default|GetNewVar_0_0) _array_index) (* (Transformation|GetActorUpVector _array_element_2) -5e+02)) _alpha) false false)))
    (:Finished
      (Utilities|FlowControl|Delay 1e+01)
      (switch Utilities|FlowControl|Switch|SwitchonETimelineDirection _direction
        (:Forward
          (Default|DisplayHUDText (Variables|Default|GetGameController) "가시 비활성화")
          (Audio|PlaySound2D "/Game/AProject/Sound/SFX/machine01_Cue.machine01_Cue" 1.0 1.0 0.0 0 0)
          (Timeline|타임라인_1 ReverseFromEnd))
        (:Backward
          (Utilities|Array|SetArrayElem _inventory _returnvalue (Utilities|Struct|MakeBP_InventoryItem (.objectname _output) (.objectdescription _output) (.additionaldescription _output) (.objectimage _output) (.objectmesh _output) (.discardable? _output) (.iskey? _output) (.keyid _output) (Utilities|GetClass self) (.discardwhenused? _output) (.inspectdistance _output) (.objectscale _output) (.lettertype _output) (.simpleletter _output) (.uifontletter _output) (.containsclue _output)))
          (|CallParentFunction))))))

(fn ConstructionScript
  (|CallParentFunction))
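; BP_ISOCSpreadGrenade is a use-action Blueprint that spawns grenades at every actor tagged "Grenade" when used.
; Its UseEvent plays a 2D bottle-opening sound, then loops over the tagged actors, spawning an enlarged BP_Grenade at each one's location and rotation.
; It then calls the parent UseEvent, and the other events and construction script add no logic of their own.
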(event EventBeginPlay
  (|CallParentFunction) ; 지금 이 노드는 비활성 상태입니다. \n핀을 끌어서 다른 노드를 연결하면 활성화됩니다.
)

(event Collision|EventActorBeginOverlap
  (params (OtherActor :type Actor%20Object%20Reference))
  (|CallParentFunction OtherActor) ; 지금 이 노드는 비활성 상태입니다. \n핀을 끌어서 다른 노드를 연결하면 활성화됩니다.
)

(event EventTick
  (params (DeltaSeconds :type Float%20%28single-precision%29))
  (|CallParentFunction DeltaSeconds) ; 지금 이 노드는 비활성 상태입니다. \n핀을 끌어서 다른 노드를 연결하면 활성화됩니다.
)

(event EventUseEvent
  (Audio|SpawnSound2D "/Game/AProject/Sound/SFX/bottleopen1_Cue.bottleopen1_Cue" 1.0 1.0 0.0 0)
  (bind _outactors (Actor|GetAllActorswithTag "Grenade"))
  (for _array_element _outactors
    (Game|SpawnActorfromClass "/Game/GrenadePack/Blueprints/BP_Grenade.BP_Grenade_C" (Math|Transform|MakeTransform (.location (Transformation|GetActorTransform _array_element)) (.rotation (Transformation|GetActorTransform _array_element)) "5.000000,5.000000,5.000000") "Undefined" 0 3.0 1e+01 0))
  (|CallParentFunction))

(fn ConstructionScript
  (|CallParentFunction))
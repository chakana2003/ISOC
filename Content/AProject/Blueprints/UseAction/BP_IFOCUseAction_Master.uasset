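; BP_IFOCUseAction_Master is, judging by its name, the base actor for item use actions.
; On UseEvent it runs the parent logic, then looks up the item at ItemInventoryIndex in the GameController's Inventory.
; Items flagged DiscardWhenUsed are removed from that index, and the action actor destroys itself in either case.
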(event EventBeginPlay
  (|CallParentFunction) ; 지금 이 노드는 비활성 상태입니다. \n핀을 끌어서 다른 노드를 연결하면 활성화됩니다.
)

(event Collision|EventActorBeginOverlap
  (params (OtherActor :type Actor%20Object%20Reference)))

(event EventTick
  (params (DeltaSeconds :type Float%20%28single-precision%29)))

(event EventUseEvent
  (|CallParentFunction)
  (if (.DiscardWhenUsed? (Utilities|Struct|BreakBP_InventoryItem (Utilities|Array|Get(acopy) (Variables|/Game/StoryAdvTemplate/Blueprints/BP_GameController.BP_GameController_C|GetInventory (Variables|Default|GetGameController)) (Variables|Default|GetItemInventoryIndex))))
    (Utilities|Array|RemoveIndex (Variables|/Game/StoryAdvTemplate/Blueprints/BP_GameController.BP_GameController_C|GetInventory (Variables|Default|GetGameController)) (Variables|Default|GetItemInventoryIndex)))
  (Actor|DestroyActor))

(fn ConstructionScript
  (|CallParentFunction))
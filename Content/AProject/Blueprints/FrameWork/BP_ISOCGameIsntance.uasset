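; Game instance Blueprint that loads intel entries from the DT_Intels data table when the game initializes.
; On Init it pairs each row name, converted to an integer, with its Title, HeadLine and LetterText column strings by index.
; Each combined entry is added to the Intels array, which is shuffled once the loop finishes to randomize its order.
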(event EventInit
  ;[0.5223 1 0.204] Intel 추출
  (bind _outrownames (DataTable|GetDataTableRowNames "/Game/AProject/CSV/DT_Intels.DT_Intels"))
  (for (_array_element _array_index) _outrownames
    (bind _returnvalue (Class|DataTableFunctionLibrary|GetDataTableColumnasString "/Game/AProject/CSV/DT_Intels.DT_Intels" "Title"))
    (bind _returnvalue_2 (Class|DataTableFunctionLibrary|GetDataTableColumnasString "/Game/AProject/CSV/DT_Intels.DT_Intels" "HeadLine"))
    (bind _returnvalue_3 (Class|DataTableFunctionLibrary|GetDataTableColumnasString "/Game/AProject/CSV/DT_Intels.DT_Intels" "LetterText"))
    (Utilities|Array|Add (Variables|Default|GetIntels) (Utilities|Struct|MakeS_CollectableIntel (Math|Conversions|ToInteger(Byte) (Utilities|String|ToString(Name) _array_element)) (Utilities|Array|Get(acopy) _returnvalue _array_index) (Utilities|Array|Get(acopy) _returnvalue_2 _array_index) (Utilities|Array|Get(acopy) _returnvalue_3 _array_index))))
  (Utilities|Array|Shuffle (Variables|Default|GetIntels)))
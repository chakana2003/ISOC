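; Game controller that carries the player's collected journal intel across the game instance and save game.
; After a short delay on BeginPlay, it copies GainIntel from the game instance into parallel title, headline and content text arrays.
; SaveGame loads or creates the "Save" slot object and rebuilds its GainIntel from those arrays before calling the parent.
; LoadGame appends saved intel to the arrays without clearing them, then calls the parent.
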(event EventBeginPlay
  (|CallParentFunction)
  (Utilities|FlowControl|Delay 0.5)
  (bind _asbp_isocgame_isntance (Utilities|Casting|CastToBP_ISOCGameIsntance (Game|GetGameInstance)))
  (for _array_element (Variables|/Game/AProject/Blueprints/FrameWork/BP_ISOCGameIsntance.BP_ISOCGameIsntance_C|GetGainIntel _asbp_isocgame_isntance)
    (Utilities|Array|Add (Variables|Default|GetCollectedJournalsTitles) (Utilities|Text|ToText(String) (.title _array_element)))
    (Utilities|Array|Add (Variables|Default|GetCollectedJournalsHeadlines) (Utilities|Text|ToText(String) (.headline _array_element)))
    (Utilities|Array|Add (Variables|Default|GetCollectedJournalsContent) (Utilities|Text|ToText(String) (.lettertext _array_element)))))

(event Collision|EventActorBeginOverlap
  (params (OtherActor :type Actor%20Object%20Reference)))

(event EventTick
  (params (DeltaSeconds :type Float%20%28single-precision%29)))

(event EventSaveGame
  (Variables|Default|SetSaving true)
  (bind _returnvalue (SaveGame|DoesSaveGameExist "Save"))
  (if _returnvalue
    (bind _returnvalue_2 (SaveGame|LoadGamefromSlot "Save"))
    (bind _asbp_save_game (Utilities|Casting|CastToBP_SaveGame _returnvalue_2))
    (Variables|Default|SetSaveGameInstance _asbp_save_game)
    (else
      (bind _returnvalue_3 (SaveGame|CreateSaveGameObject (Variables|Default|GetSaveGameClass)))
      (Variables|Default|SetSaveGameInstance (.AsBP%20Save%20Game (Utilities|Casting|CastToBP_SaveGame _returnvalue_3)))))
  (bind _asbp_isocsave_game (Utilities|Casting|CastToBP_ISOCSaveGame (Variables|Default|GetSaveGameInstance)))
  (Utilities|Array|Clear (Variables|/Game/AProject/Blueprints/FrameWork/BP_ISOCSaveGame.BP_ISOCSaveGame_C|GetGainIntel _asbp_isocsave_game))
  (for (_array_element _array_index) (Variables|Default|GetCollectedJournalsTitles)
    (Utilities|Array|Add (Variables|/Game/AProject/Blueprints/FrameWork/BP_ISOCSaveGame.BP_ISOCSaveGame_C|GetGainIntel _asbp_isocsave_game) (Utilities|Struct|MakeS_CollectableIntel 0 (Utilities|String|ToString(Text) _array_element) (Utilities|String|ToString(Text) (Utilities|Array|Get(acopy) (Variables|Default|GetCollectedJournalsHeadlines) _array_index)) (Utilities|String|ToString(Text) (Utilities|Array|Get(acopy) (Variables|Default|GetCollectedJournalsContent) _array_index)))))
  (|CallParentFunction))

(event EventLoadGame
  (bind _returnvalue (SaveGame|LoadGamefromSlot "Save"))
  (bind _asbp_save_game (Utilities|Casting|CastToBP_SaveGame _returnvalue))
  (bind _output_get (Variables|Default|SetSaveGameInstance _asbp_save_game))
  (bind _asbp_isocsave_game (Utilities|Casting|CastToBP_ISOCSaveGame _output_get))
  (for _array_element (Variables|/Game/AProject/Blueprints/FrameWork/BP_ISOCSaveGame.BP_ISOCSaveGame_C|GetGainIntel _asbp_isocsave_game)
    (Utilities|Array|Add (Variables|Default|GetCollectedJournalsTitles) (Utilities|Text|ToText(String) (.title _array_element)))
    (Utilities|Array|Add (Variables|Default|GetCollectedJournalsHeadlines) (Utilities|Text|ToText(String) (.headline _array_element)))
    (Utilities|Array|Add (Variables|Default|GetCollectedJournalsContent) (Utilities|Text|ToText(String) (.lettertext _array_element))))
  (|CallParentFunction))

(fn ConstructionScript
  (|CallParentFunction))
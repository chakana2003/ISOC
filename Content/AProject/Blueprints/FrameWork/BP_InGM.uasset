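; In-game game mode that procedurally builds the room layout at BeginPlay when the game instance flags gameplay.
; A randomly chosen BP_PlayRoom starts room numbering, then numbered rooms are linked by doors whose KeyID matches the room each opens into.
; Remaining slots get walls, and an extra final room is spawned on a free side behind an unlocked door.
; A last pass removes walls that overlap at the same location.
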(event EventBeginPlay
  (bind _asbp_isocgame_isntance (Utilities|Casting|CastToBP_ISOCGameIsntance (Game|GetGameInstance)))
  (if (Variables|/Game/AProject/Blueprints/FrameWork/BP_ISOCGameIsntance.BP_ISOCGameIsntance_C|GetIsGamePlay _asbp_isocgame_isntance)
    (bind _outactors (Actor|GetAllActorsOfClass "/Game/AProject/Blueprints/BP_PlayRoom.BP_PlayRoom_C"))
    (bind _output_get (Variables|Default|SetPlayRooms _outactors))
    (Utilities|Array|Shuffle _output_get)
    (bind _returnstagenum (Default|CreateRoomNumberandOutWall (Utilities|Array|Get(acopy) _output_get) 1))
    (CallFunction|CreateDoorsandWalls (Variables|Default|GetPlayRooms))
    (CallFunction|CreateLastRoom (Variables|Default|GetPlayRooms) _returnstagenum)
    ;[1 0.2977 0.9375] 의도하진 않았지만 자연스레 방의 구조가 만들어짐
    (bind _outactors_2 (Actor|GetAllActorsOfClass "/Game/AProject/Blueprints/Props/Wall/BP_Wall.BP_Wall_C"))
    (bind _output_get_2 (Variables|Default|SetNewVar_0 _outactors_2))
    (bind _output_get_3 (Variables|Default|SetNewVar_1 _outactors_2))
    (for _array_element _output_get_2
      (for _array_element_2 _output_get_3
        (if (not (== _array_element_2 _array_element))
          (if (Math|Vector|Equal(Vector) (Transformation|GetActorLocation _array_element_2) (Transformation|GetActorLocation _array_element) 1.0)
            (Utilities|Array|AddUnique (Variables|Default|GetNewVar_2) _array_element_2)))))
    (bind _arrayelement (Utilities|Array|ReverseforEachLoop (Variables|Default|GetNewVar_2))
      (:LoopBody
        (Actor|DestroyActor _arrayelement)))))

(event EventTick
  (params (DeltaSeconds :type Float%20%28single-precision%29)))

(fn ConstructionScript)

(fn CreateLastRoom
  (params (Array :type Array%20of%20BP%20Play%20Room%20Object%20References) (StageNum :type Integer))
  (bind _enabledirection (LocalVariables|GetEnableDirection))
  (bind _output (Utilities|Array|Get(acopy) _enabledirection))
  (Utilities|Array|Shuffle Array)
  (bind _array_element (Utilities|Array|ForEachLoopwithBreak Array :!label _label)
    (:LoopBody
      (bind _keys (Utilities|Map|Keys (Variables|/Game/AProject/Blueprints/BP_PlayRoom.BP_PlayRoom_C|GetAroundRooms _array_element)))
      (for _array_element_2 _keys
        (Utilities|IsValid (.Value (Utilities|Map|Find (Variables|/Game/AProject/Blueprints/BP_PlayRoom.BP_PlayRoom_C|GetAroundRooms _array_element) _array_element_2))
          (:Is%20Not%20Valid
            (Utilities|Array|Add (LocalVariables|GetEnableDirection) _array_element_2))))
      (if (Utilities|Array|IsValidIndex (LocalVariables|GetEnableDirection))
        (LocalVariables|SetTargetRoom _array_element)
        (goto _label Break)))
    (:Completed
      (Utilities|Array|Shuffle _enabledirection)
      (bind _returnvalue (Game|SpawnActorfromClass "/Game/AProject/Blueprints/BP_PlayRoom.BP_PlayRoom_C" (Utilities|Select :Index _output :NewEnumerator0 (Math|Transform|MakeTransform (+ (Transformation|GetActorLocation (LocalVariables|GetTargetRoom)) "2000.000000, 0,0.000000") "0, 0, 0" "1,1,1") :NewEnumerator1 (Math|Transform|MakeTransform (Transformation|GetActorLocation (LocalVariables|GetTargetRoom)) "0,180.000000, 0" "1,1,1") :NewEnumerator2 (Math|Transform|MakeTransform (+ (Transformation|GetActorLocation (LocalVariables|GetTargetRoom)) "1000.000000,1000.000000, 0") "0,90.000000,0.000000" "1,1,1") :NewEnumerator3 (Math|Transform|MakeTransform (+ (Transformation|GetActorLocation (LocalVariables|GetTargetRoom)) "1000.000000,-1000.000000, 0") "0,-90.000000, 0" "1,1,1")) "Undefined" 0 0))
      (Default|CreateRoomNumberandOutWall _returnvalue StageNum)
      (Default|DestroyWall _returnvalue "NewEnumerator1")
      (for _array_element_3 (Actor|GetComponentsbyTag _returnvalue "/Script/Engine.SceneComponent" "N")
        (bind _returnvalue_2 (Game|SpawnActorfromClass "/Game/AProject/Blueprints/Props/Wall/BP_Wall.BP_Wall_C" (Math|Transform|MakeTransform "0, 0, 0" "0, 0, 0" "1,1,1") "AlwaysSpawn" 0 true 0))
        (Transformation|AttachComponentToComponent _returnvalue_2 _array_element_3 "None" "KeepRelative" "KeepRelative" "KeepRelative" true))
      (for _array_element_4 (Actor|GetComponentsbyTag _returnvalue "/Script/Engine.SceneComponent" "E")
        (bind _returnvalue_3 (Game|SpawnActorfromClass "/Game/AProject/Blueprints/Props/Wall/BP_Wall.BP_Wall_C" (Math|Transform|MakeTransform "0, 0, 0" "0, 0, 0" "1,1,1") "AlwaysSpawn" 0 true 0))
        (Transformation|AttachComponentToComponent _returnvalue_3 _array_element_4 "None" "KeepRelative" "KeepRelative" "KeepRelative" true))
      (for _array_element_5 (Actor|GetComponentsbyTag _returnvalue "/Script/Engine.SceneComponent" "W")
        (bind _returnvalue_4 (Game|SpawnActorfromClass "/Game/AProject/Blueprints/Props/Wall/BP_Wall.BP_Wall_C" (Math|Transform|MakeTransform "0, 0, 0" "0, 0, 0" "1,1,1") "AlwaysSpawn" 0 true 0))
        (Transformation|AttachComponentToComponent _returnvalue_4 _array_element_5 "None" "KeepRelative" "KeepRelative" "KeepRelative" true))
      (bind _returntargetindex (Default|DestroyOneWall (LocalVariables|GetTargetRoom) _output (Math|Random|RandomIntegerinRange 0 (- (Utilities|Array|Length (Actor|GetComponentsbyTag (LocalVariables|GetTargetRoom) "/Script/Engine.SceneComponent" (Utilities|Select :Index _output :NewEnumerator0 "N" :NewEnumerator1 "S" :NewEnumerator2 "E" :NewEnumerator3 "W"))) 1))))
      (bind _returnvalue_5 (Game|SpawnActorfromClass "/Game/AProject/Blueprints/Props/BP_ISOCInteractiveDoor.BP_ISOCInteractiveDoor_C" (Math|Transform|MakeTransform "0, 0, 0" "0, 0, 0" "1,1,1") "Undefined" 0 0))
      (Transformation|AttachComponentToComponent _returnvalue_5 (Utilities|Array|Get(acopy) (Actor|GetComponentsbyTag (LocalVariables|GetTargetRoom) "/Script/Engine.SceneComponent" (Utilities|Select :Index _output :NewEnumerator0 "N" :NewEnumerator1 "S" :NewEnumerator2 "E" :NewEnumerator3 "W")) _returntargetindex) "None" "KeepRelative" "KeepRelative" "KeepRelative" true)
      (Variables|/Game/StoryAdvTemplate/Blueprints/MasterBlueprints/Doors/BP_Master_Door.BP_Master_Door_C|SetKeyID _returnvalue_5 10)
      (Variables|/Game/StoryAdvTemplate/Blueprints/MasterBlueprints/Doors/BP_Master_Door.BP_Master_Door_C|SetisLocked? _returnvalue_5 false))))

(fn CreateDoorsandWalls
  (params (Array :type Array%20of%20BP%20Play%20Room%20Object%20References))
  (bind _passrooms (LocalVariables|GetPassRooms))
  (bind _array_element (Utilities|Array|ForEachLoopwithBreak Array :!label _label)
    (:LoopBody
      (if (== (Variables|/Game/AProject/Blueprints/BP_PlayRoom.BP_PlayRoom_C|GetRoomNum _array_element) 1)
        (Utilities|Array|Add (LocalVariables|GetTargetRoomsRef) _array_element)
        (goto _label Break)))
    (:Completed
      (for _index (range 2 9)
        (Utilities|Map|Clear (LocalVariables|GetPassRooms))
        (for _array_element_2 (LocalVariables|GetTargetRoomsRef)
          (bind _keys (Utilities|Map|Keys (Variables|/Game/AProject/Blueprints/BP_PlayRoom.BP_PlayRoom_C|GetAroundRooms _array_element_2)))
          (bind _array_element_3 (Utilities|Array|ForEachLoopwithBreak _keys :!label _label_2)
            (:LoopBody
              (Utilities|IsValid (.Value (Utilities|Map|Find (Variables|/Game/AProject/Blueprints/BP_PlayRoom.BP_PlayRoom_C|GetAroundRooms _array_element_2) _array_element_3))
                (:Is%20Valid
                  (if (== (Variables|/Game/AProject/Blueprints/BP_PlayRoom.BP_PlayRoom_C|GetRoomNum (.Value (Utilities|Map|Find (Variables|/Game/AProject/Blueprints/BP_PlayRoom.BP_PlayRoom_C|GetAroundRooms _array_element_2) _array_element_3))) _index)
                    (Utilities|Map|Add (LocalVariables|GetPassRooms) _array_element_2 _array_element_3)
                    (goto _label_2 Break)))))))
        (bind _keys_2 (Utilities|Map|Keys _passrooms))
        (Utilities|Array|Shuffle _keys_2)
        (bind _output_get (LocalVariables|SetTargetRoom (Utilities|Array|Get(acopy) _keys_2)))
        (bind _output_get_2 (LocalVariables|SetFinidComponents (Actor|GetComponentsbyTag _output_get "/Script/Engine.SceneComponent" (Utilities|Select :Index (.Value (Utilities|Map|Find _passrooms _output_get)) :NewEnumerator0 "N" :NewEnumerator1 "S" :NewEnumerator2 "E" :NewEnumerator3 "W"))))
        (Utilities|Array|Shuffle _output_get_2)
        (for (_array_element_4 _array_index) (LocalVariables|GetFinidComponents)
          (if (== _array_index 0)
            (bind _returnvalue (Game|SpawnActorfromClass "/Game/AProject/Blueprints/Props/BP_ISOCInteractiveDoor.BP_ISOCInteractiveDoor_C" (Math|Transform|MakeTransform "0, 0, 0" "0, 0, 0" "1,1,1") "AlwaysSpawn" _output_get 0))
            (Transformation|AttachComponentToComponent _returnvalue _array_element_4 "None" "KeepRelative" "KeepRelative" "KeepRelative" false)
            (Utilities|Array|Add (LocalVariables|GetDoorPositionRef) _array_element_4)
            (Variables|/Game/StoryAdvTemplate/Blueprints/MasterBlueprints/Doors/BP_Master_Door.BP_Master_Door_C|SetKeyID _returnvalue _index)))
        (Utilities|Array|AddUnique (LocalVariables|GetTargetRoomsRef) (.Value (Utilities|Map|Find (Variables|/Game/AProject/Blueprints/BP_PlayRoom.BP_PlayRoom_C|GetAroundRooms _output_get) (.Value (Utilities|Map|Find _passrooms _output_get)))))
        (Default|DestroyComponents (.Value (Utilities|Map|Find (Variables|/Game/AProject/Blueprints/BP_PlayRoom.BP_PlayRoom_C|GetAroundRooms _output_get) (.Value (Utilities|Map|Find _passrooms _output_get)))) (.Value (Utilities|Map|Find _passrooms _output_get))))
      (for _array_element_5 Array
        (for _array_element_6 (Actor|GetComponentsbyTag _array_element_5 "/Script/Engine.SceneComponent" "WallPlace")
          (if (== (Utilities|Array|FindItem (LocalVariables|GetDoorPositionRef) _array_element_6) -1)
            (bind _returnvalue_2 (Game|SpawnActorfromClass "/Game/AProject/Blueprints/Props/Wall/BP_Wall.BP_Wall_C" (Math|Transform|MakeTransform "0, 0, 0" "0, 0, 0" "1,1,1") "AlwaysSpawn" _array_element_5 (not (Components|ComponentHasTag _array_element_6 "Outside")) 0))
            (Transformation|AttachComponentToComponent _returnvalue_2 _array_element_6 "None" "KeepRelative" "KeepRelative" "KeepRelative" true)))))))
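; BP_EndMissile is an actor that animates a missile mesh flying to the actor's origin, apparently as an end-of-game event.
; On BeginPlay it stores the mesh's relative start location and turns it toward the origin with a 90-degree rotation offset.
; The ShootMissile timeline, rate-scaled by LoopTime, lerps the mesh inward without sweep.
; On finish it only prints a "ResetGame" message; no reset logic exists here.
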(event EventBeginPlay
  (bind _missilemesh (Variables|Default|GetMissileMesh))
  (bind _relativelocation (Variables|/Script/Engine.SceneComponent|GetRelativeLocation _missilemesh))
  (Variables|Default|SetStartRelativeLocation _relativelocation)
  (Transformation|SetRelativeRotation _missilemesh (Math|Rotator|CombineRotators (Math|Rotator|FindLookatRotation _relativelocation (Math|Vector|MakeVector 0.0 0.0 0.0)) "0.000000,0.000000,90.000000") false false)
  (Components|Timeline|SetPlayRate (Variables|Default|GetShootMissile) (/ 1.0 (Variables|Default|GetLoopTime)))
  (bind _alpha (Timeline|ShootMissile PlayFromStart)
    (:Update
      (Transformation|SetRelativeLocation (Variables|Default|GetMissileMesh) (Math|Vector|Lerp(Vector) (Variables|Default|GetStartRelativeLocation) "0, 0, 0" _alpha) false false))
    (:Finished
      (Development|PrintString "ResetGame" true true "(R=1.000000,G=0.089822,B=0.000000,A=1.000000)" 3e+01))))

(event Collision|EventActorBeginOverlap
  (params (OtherActor :type Actor%20Object%20Reference)))

(event EventTick
  (params (DeltaSeconds :type Float%20%28single-precision%29)))

(fn ConstructionScript)
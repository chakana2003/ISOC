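; Menu pawn whose camera frames the player character and the end missile, applying the possessing BP_InPC's saturation as post-process settings.
; BeginPlay finds both actors and records the initial camera-to-missile distance.
; Tick aims the camera at their midpoint, blending in a rotation offset based on normalized missile distance.
; It also refreshes item and close-up locations from four scene components every frame.
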(event EventBeginPlay
  (Utilities|FlowControl|Sequence
    (:then_0
      (bind _outactors (Actor|GetAllActorsOfClass "/Game/AProject/Blueprints/BP_EndMissile.BP_EndMissile_C"))
      (if (Utilities|Array|IsValidIndex _outactors)
        (bind _output_get (Variables|Default|SetEndMissileRef (Utilities|Array|Get(acopy) _outactors)))
        (Variables|Default|SetInitMaxLengh (Math|Vector|VectorLength (- (Transformation|GetWorldLocation (Variables|/Game/AProject/Blueprints/BP_EndMissile.BP_EndMissile_C|GetMissileMesh _output_get)) (Transformation|GetWorldLocation (Variables|Default|GetCamera)))))))
    (:then_1
      (bind _outactors_2 (Actor|GetAllActorsOfClass "/Game/AProject/Blueprints/BP_ISOCPlayerCharacter.BP_ISOCPlayerCharacter_C"))
      (if (Utilities|Array|IsValidIndex _outactors_2)
        (Variables|Default|SetCharacterRef (Utilities|Array|Get(acopy) _outactors_2))))))

(event Collision|EventActorBeginOverlap
  (params (OtherActor :type Actor%20Object%20Reference)))

(event EventTick
  (params (DeltaSeconds :type Float%20%28single-precision%29))
  (bind _endmissileref (Variables|Default|GetEndMissileRef))
  (bind _camera (Variables|Default|GetCamera))
  (bind _returnvalue (Transformation|GetWorldLocation _camera))
  (bind _missilemesh (Variables|/Game/AProject/Blueprints/BP_EndMissile.BP_EndMissile_C|GetMissileMesh _endmissileref))
  (bind _returnvalue_2 (Transformation|GetWorldLocation _missilemesh))
  (|CallParentFunction DeltaSeconds)
  (Utilities|FlowControl|Sequence
    (:then_0
      (Utilities|IsValid _endmissileref
        (:Is%20Valid
          (Transformation|SetWorldRotation _camera (Math|Rotator|CombineRotators (Math|Rotator|FindLookatRotation _returnvalue (/ (+ _returnvalue_2 (Transformation|GetActorLocation (Variables|Default|GetCharacterRef))) 2.0)) (Math|Rotator|Lerp(Rotator) "0,20.000000, 0" "0,40.000000, 0" (Math|Float|Clamp(Float) (Math|Float|NormalizetoRange (Math|Vector|VectorLength (- _returnvalue _returnvalue_2)) 1e+05 (Variables|Default|GetInitMaxLengh))))) false false))))
    (:then_1
      (Variables|Default|SetSelectedItemLocation (Transformation|GetWorldLocation (Variables|Default|GetScene2)))
      (Variables|Default|SetSecondItemLocation (Transformation|GetWorldLocation (Variables|Default|GetScene)))
      (Variables|Default|SetLastItemLocation (Transformation|GetWorldLocation (Variables|Default|GetScene3)))
      (Variables|Default|SetCloseUpLocation (Transformation|GetWorldLocation (Variables|Default|GetScene1))))))

(event EventPossessed
  (params (NewController :type Controller%20Object%20Reference))
  (|CallParentFunction NewController)
  (bind _asbp_in_pc (Utilities|Casting|CastToBP_InPC NewController))
  (Variables|/Script/Engine.CameraComponent|SetPostProcessSettings (Variables|Default|GetCamera) (Utilities|Struct|MakePostProcessSettings (Variables|/Game/AProject/Blueprints/FrameWork/BP_InPC.BP_InPC_C|GetCharacterSaturation _asbp_in_pc))))

(fn ConstructionScript
  (|CallParentFunction))
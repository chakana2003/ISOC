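; BP_ISOCMaster_Drawer is a master drawer prop Blueprint, with a SpawnProps event scaffolded for keys, stones and intel.
; SpawnProps runs three sequenced passes: counted loops for keys and stones, then a loop over IntelIndexes.
; The intel pass searches the game instance's Intels for a matching IntelCode and breaks on a hit.
; The loops spawn nothing yet, and the construction script only calls its parent.
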(event EventBeginPlay
  (|CallParentFunction) ; 지금 이 노드는 비활성 상태입니다. \n핀을 끌어서 다른 노드를 연결하면 활성화됩니다.
)

(event Collision|EventActorBeginOverlap
  (params (OtherActor :type Actor%20Object%20Reference)))

(event EventTick
  (params (DeltaSeconds :type Float%20%28single-precision%29)))

(event EventSpawnProps
  (params (KeyCount :type Integer) (StoneCount :type Integer) (IntelIndexes :type Array%20of%20Integers))
  (Utilities|FlowControl|Sequence
    (:then_0
      (if (> KeyCount 0)
        (for _index (range 1 KeyCount)
          _)))
    (:then_1
      (if (> StoneCount 0)
        (for _index_2 (range 1 StoneCount)
          _)))
    (:then_2
      (if (Utilities|Array|IsValidIndex IntelIndexes)
        (for (_ _array_index) IntelIndexes
          (bind _asbp_isocgame_isntance (Utilities|Casting|CastToBP_ISOCGameIsntance (Game|GetGameInstance)))
          (bind _array_element (Utilities|Array|ForEachLoopwithBreak (Variables|/Game/AProject/Blueprints/FrameWork/BP_ISOCGameIsntance.BP_ISOCGameIsntance_C|GetIntels _asbp_isocgame_isntance) :!label _label)
            (:LoopBody
              (if (== (.intelcode _array_element) _array_index)
                (goto _label Break)))))))))

(fn ConstructionScript
  (|CallParentFunction))
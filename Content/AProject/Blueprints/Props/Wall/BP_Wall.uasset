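; BP_Wall is a modular wall prop for BP_PlayRoom that shows a random wall or window mesh.
; The construction script picks the mesh from Windows or Walls based on CanHaveWindow.
; UpdateWall derives MySide from its signed yaw relative to the parent room, registers missing sides in WallInfo, and swaps to a random wall for one specific state.
; An unconnected branch checks neighboring rooms for RoomNum 10 to choose wall or window.
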(event Custom|UpdateWall
  (bind _returnvalue (Actor|GetAttachParentActor))
  (bind _returnvalue_2 (Transformation|GetActorTransform))
  (bind _returnvalue_3 (Math|Vector|MakeVector 1.0 0.0 0.0))
  (bind _returnvalue_4 (Actor|GetAttachParentActor))
  (bind _walls (Variables|Default|GetWalls))
  (bind (_x _y) (Math|Vector|BreakVector _returnvalue_3))
  (bind _returnvalue_5 (Transformation|GetActorTransform _returnvalue_4))
  (bind _returnvalue_6 (Math|Transform|MakeRelativeTransform _returnvalue_2 _returnvalue_5))
  (bind _returnvalue_7 (Math|Vector|GetForwardVector (.rotation _returnvalue_6)))
  (bind _returnvalue_8 (Math|Vector|DotProduct _returnvalue_3 _returnvalue_7))
  (bind (_x_2 _y_2) (Math|Vector|BreakVector _returnvalue_7))
  (bind _returnvalue_9 (Class|KismetMathLibrary|DegAcos _returnvalue_8))
  (bind _returnvalue_10 (* _y _x_2))
  (bind _returnvalue_11 (* _x _y_2))
  (bind _returnvalue_12 (* _returnvalue_9 -1.0))
  (bind _returnvalue_13 (+ _returnvalue_11 _returnvalue_10))
  (bind _returnvalue_14 (<= _returnvalue_13 0.0))
  (bind _returnvalue_15 (select _returnvalue_14 _returnvalue_9 _returnvalue_12))
  (Utilities|IsValid _returnvalue
    (:Is%20Valid
      (if (== _returnvalue_15 0.0)
        (Variables|Default|SetMySide "NewEnumerator1")
        (elif (> _returnvalue_15 0.0)
          (Variables|Default|SetMySide "NewEnumerator2")
          (elif (> _returnvalue_15 -1.3e+02)
            (Variables|Default|SetMySide "NewEnumerator3")
            (else
              (Variables|Default|SetMySide "NewEnumerator0")))))
      (Utilities|FlowControl|Sequence
        (:then_0
          (bind _asbp_play_room (Utilities|Casting|CastToBP_PlayRoom _returnvalue))
          (if (not (.ReturnValue (Utilities|Map|Find (Variables|/Game/AProject/Blueprints/BP_PlayRoom.BP_PlayRoom_C|GetWallInfo _asbp_play_room) (Variables|Default|GetMySide))))
            (Utilities|Map|Add (Variables|/Game/AProject/Blueprints/BP_PlayRoom.BP_PlayRoom_C|GetWallInfo _asbp_play_room) (Variables|Default|GetMySide) "NewEnumerator1")))
        (:then_1
          (bind _asbp_play_room_2 (Utilities|Casting|CastToBP_PlayRoom (Actor|GetAttachParentActor)))
          (if (.ReturnValue (Utilities|Map|Find (Variables|/Game/AProject/Blueprints/BP_PlayRoom.BP_PlayRoom_C|GetWallInfo _asbp_play_room_2) (Variables|Default|GetMySide)))
            (if (Utilities|Enum|Equal(Enum) (.Value (Utilities|Map|Find (Variables|/Game/AProject/Blueprints/BP_PlayRoom.BP_PlayRoom_C|GetWallInfo _asbp_play_room_2) (Variables|Default|GetMySide))) "NewEnumerator3")
              (Components|StaticMesh|SetStaticMesh (Variables|Debug|GetStaticMeshComponent) (Utilities|Array|Get(acopy) _walls (Math|Random|RandomIntegerinRange 0 (- (Utilities|Array|Length _walls) 1)))))))))))

(event EventBeginPlay)

(event Collision|EventActorBeginOverlap
  (params (OtherActor :type Actor%20Object%20Reference)))

(event EventTick
  (params (DeltaSeconds :type Float%20%28single-precision%29)))

(fn ConstructionScript
  (bind _staticmeshcomponent (Variables|Debug|GetStaticMeshComponent))
  (bind _windows (Variables|Default|GetWindows))
  (bind _walls (Variables|Default|GetWalls))
  (if (Variables|Default|GetCanHaveWindow)
    (Components|StaticMesh|SetStaticMesh _staticmeshcomponent (Utilities|Array|Get(acopy) _windows (Math|Random|RandomIntegerinRange 0 (- (Utilities|Array|Length _windows) 1))))
    (else
      (Components|StaticMesh|SetStaticMesh _staticmeshcomponent (Utilities|Array|Get(acopy) _walls (Math|Random|RandomIntegerinRange 0 (- (Utilities|Array|Length _walls) 1)))))))
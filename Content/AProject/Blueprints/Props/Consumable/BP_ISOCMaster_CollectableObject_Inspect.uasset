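; Master Blueprint for an inspectable collectable prop that simulates physics only near the player and plays impact sounds.
; BeginPlay caches the player character after a startup delay.
; Tick checks player distance, using two opposing Gates to switch the object's physics only when it crosses the range threshold.
; Hard hits play a sound through a DoOnce, armed after startup and reset after a short cooldown.
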(event OnComponentHit(Object)
  (params (HitComponent :type Primitive%20Component%20Object%20Reference) (OtherActor :type Actor%20Object%20Reference) (OtherComp :type Primitive%20Component%20Object%20Reference) (NormalImpulse :type Vector :default "0, 0, 0") (Hit :type Hit%20Result%20Structure%20%28by%20ref%29))
  (if (> (Math|Vector|VectorLength NormalImpulse) 4e+03)
    (Utilities|FlowControl|DoOnce true :!label _label
      (:Completed
        (Audio|PlaySoundatLocation (Variables|Setup|GetHitSound) (Transformation|GetWorldLocation (Variables|Default|GetObject)) "0, 0, 0" 1.0 1.0 0.0 0 0 0)
        (Utilities|FlowControl|Delay 1.0)
        (goto _label Reset)))))

(event EventBeginPlay
  (|CallParentFunction)
  (Utilities|FlowControl|Delay 5.0)
  (bind _outactors (Actor|GetAllActorsOfClass "/Game/AProject/Blueprints/BP_ISOCPlayerCharacter.BP_ISOCPlayerCharacter_C"))
  (Variables|Default|SetCharacterRef (Utilities|Array|Get(acopy) _outactors))
  (Utilities|FlowControl|Delay 2.0)
  (Utilities|FlowControl|DoOnce true) ; enters at Reset
)

(event Collision|EventActorBeginOverlap
  (params (OtherActor :type Actor%20Object%20Reference)))

(event EventTick
  (params (DeltaSeconds :type Float%20%28single-precision%29))
  (bind _characterref (Variables|Default|GetCharacterRef))
  (bind _object (Variables|Default|GetObject))
  (bind _returnvalue (Transformation|GetActorLocation _characterref))
  (bind _returnvalue_2 (Transformation|GetWorldLocation _object))
  (bind _returnvalue_3 (- _returnvalue _returnvalue_2))
  (bind _returnvalue_4 (Math|Vector|VectorLength _returnvalue_3))
  (bind _returnvalue_5 (< _returnvalue_4 1e+03))
  (Utilities|IsValid _characterref
    (:Is%20Valid
      (if _returnvalue_5
        (Utilities|FlowControl|Sequence
          (:then_0
            (Utilities|FlowControl|Gate true :!label _label
              (:Exit
                (Variables|Default|SetSimulatePhysics _returnvalue_5)
                (Physics|SetSimulatePhysics (Variables|Default|GetObject) _returnvalue_5))))
          (:then_1
            (goto _label Close))
          (:then_2
            (goto _label_2 Open)))
        (else
          (Utilities|FlowControl|Sequence
            (:then_0
              (Utilities|FlowControl|Gate true :!label _label_2
                (:Exit
                  (Variables|Default|SetSimulatePhysics _returnvalue_5)
                  (Physics|SetSimulatePhysics (Variables|Default|GetObject) _returnvalue_5))))
            (:then_1
              (goto _label Open))
            (:then_2
              (goto _label_2 Close))))))))

(fn ConstructionScript
  (|CallParentFunction))
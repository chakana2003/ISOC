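; Missile actor for what appears to be a menu ending sequence, which flies into a big impact and then loads Map_ISOCGame.
; Fire aims the mesh and lerps it to the actor origin over LoopTime via a timeline, then broadcasts THEGREATIMPACT.
; Unless CatchPortal is set, DOIMPACT spawns huge shockwave emitters and bomb sounds.
; It also ramps camera shake on the first Chameleon actor, opening the level when that ramp ends.
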(event Custom|DOIMPACT
  (bind _missilemesh (Variables|Default|GetMissileMesh))
  (bind _returnvalue (Transformation|GetWorldLocation _missilemesh))
  (if (not (Variables|Default|GetCatchPortal))
    (Utilities|FlowControl|Sequence
      (:then_0
        (Effects|SpawnEmitteratLocation "/Game/Explosions/Particles/P_FlareShimmer2.P_FlareShimmer2" _returnvalue "0, 0, 0" "500.000000,500.000000,500.000000" true "AutoRelease")
        (Audio|PlaySound2D "/Game/AProject/Sound/SFX/46414__erh__asynth-30-bomb.46414__erh__asynth-30-bomb" 1.0 1.0 0.0 0 0)
        (bind _outactors (Actor|GetAllActorsOfClass "/Game/Chameleon/Chameleon.Chameleon_C"))
        (Variables|/Game/Chameleon/Chameleon.Chameleon_C|SetCamera%20Shake (Utilities|Array|Get(acopy) _outactors) true)
        (bind _alpha (Timeline|타임라인_0 PlayFromStart)
          (:Update
            (Variables|/Game/Chameleon/Chameleon.Chameleon_C|SetCamera%20Shake%20Power%20%28X%29 (Utilities|Array|Get(acopy) _outactors) (Math|Float|Lerp 0.0 0.05 _alpha))
            (Variables|/Game/Chameleon/Chameleon.Chameleon_C|SetCamera%20Shake%20Power%20%28Y%29 (Utilities|Array|Get(acopy) _outactors) (Math|Float|Lerp 0.0 0.05 _alpha)))
          (:Finished
            (CallFunction|TIMELOOP))))
      (:then_1
        (Effects|SpawnEmitteratLocation "/Game/Explosions/Particles/P_shockwave7.P_shockwave7" _returnvalue "90.000000, 0, 0" "500.000000,500.000000,500.000000")
        (Utilities|FlowControl|Delay 2.0)
        (Audio|PlaySound2D "/Game/AProject/Sound/SFX/261216__superwarrior543__bomb.261216__superwarrior543__bomb" 1.0 1.0 0.0 0 0)
        (Effects|SpawnEmitteratLocation "/Game/Explosions/Particles/P_shockwave6.P_shockwave6" _returnvalue "90.000000, 0, 0" "500.000000,500.000000,500.000000"))
      (:then_2
        (Effects|SpawnEmitteratLocation "/Game/Explosions/Particles/P_shockwave8.P_shockwave8" _returnvalue "90.000000, 0, 0" "500.000000,500.000000,500.000000"))
      (:then_3
        (Effects|SpawnEmitteratLocation "/Game/Explosions/Particles/P_shockwave9.P_shockwave9" _returnvalue "90.000000, 0, 0" "500.000000,500.000000,500.000000")))))

(event Custom|TIMELOOP
  (Game|OpenLevel(byName) "Map_ISOCGame"))

(event Custom|Fire
  (bind _missilemesh (Variables|Default|GetMissileMesh))
  (bind _relativelocation (Variables|/Script/Engine.SceneComponent|GetRelativeLocation _missilemesh))
  (EventDispatchers|BindEventtoTHEGREATIMPACT (delegate Custom|DOIMPACT))
  (Variables|Default|SetStartRelativeLocation _relativelocation)
  (Transformation|SetRelativeRotation _missilemesh (Math|Rotator|CombineRotators (Math|Rotator|FindLookatRotation _relativelocation (Math|Vector|MakeVector 0.0 0.0 0.0)) "0.000000,0.000000,90.000000") false false)
  (Components|Timeline|SetPlayRate (Variables|Default|GetShootMissile) (/ 1.0 (Variables|Default|GetLoopTime)))
  (bind _alpha (Timeline|ShootMissile PlayFromStart)
    (:Update
      (Transformation|SetRelativeLocation (Variables|Default|GetMissileMesh) (Math|Vector|Lerp(Vector) (Variables|Default|GetStartRelativeLocation) "0, 0, 0" _alpha) false false))
    (:Finished
      (Default|CallTHEGREATIMPACT))))

(fn ConstructionScript)
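; End-of-game portal that moves the player to a fixed ending location on capsule overlap.
; BeginPlay caches scene references, enables Chameleon radial blur and plays portal effects and sounds.
; Tick scales blur width with player proximity inside a short radius.
; Overlap flags the end missile and game controller, zeroes the directional light, disables toon shading, stops music and starts the player's camera sequence.
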(event OnComponentBeginOverlap(Capsule)
  (params (OverlappedComponent :type Primitive%20Component%20Object%20Reference) (OtherActor :type Actor%20Object%20Reference) (OtherComp :type Primitive%20Component%20Object%20Reference) (OtherBodyIndex :type Integer) (bFromSweep :type Boolean) (SweepResult :type Hit%20Result%20Structure%20%28by%20ref%29))
  (bind _asbp_isocplayer_character (Utilities|Casting|CastToBP_ISOCPlayerCharacter OtherActor))
  (Variables|/Game/AProject/Blueprints/BP_EndMissile.BP_EndMissile_C|SetCatchPortal (Variables|Default|GetEndMissile) true)
  (Transformation|SetActorLocation _asbp_isocplayer_character "-26801.000000,24364.000000,-30104.382813" false false)
  (Rendering|Components|Light|SetIntensity (Variables|/Script/Engine.Light|GetLightComponent (Variables|Default|GetDirectLight)) 0.0)
  (Default|Clear _asbp_isocplayer_character)
  (Default|BeginCameraPlay _asbp_isocplayer_character true)
  (Variables|/Game/StoryAdvTemplate/Blueprints/BP_GameController.BP_GameController_C|SetGameFinish (Variables|Default|GetGameControllerRef) true)
  (Variables|/Game/Chameleon/Chameleon.Chameleon_C|SetToon%20Shading (Variables|Default|GetChameleonRef) false)
  (Audio|Components|Audio|Stop (Variables|/Game/AProject/Blueprints/BP_ISOCPlayerCharacter.BP_ISOCPlayerCharacter_C|GetCurrentMusic _asbp_isocplayer_character))
  (Audio|PlaySound2D "/Game/AProject/Sound/SFX/330724__robinhood76__06145-futuristic-magnetic-gate.330724__robinhood76__06145-futuristic-magnetic-gate" 1.0 1.0 0.0 0 0))

(event EventBeginPlay
  (Utilities|FlowControl|Sequence
    (:then_0
      (bind _outactors (Actor|GetAllActorsOfClass "/Game/Chameleon/Chameleon.Chameleon_C"))
      (Variables|Default|SetChameleonRef (Utilities|Array|Get(acopy) _outactors)))
    (:then_1
      (bind _outactors_2 (Actor|GetAllActorsOfClass "/Game/AProject/Blueprints/BP_ISOCPlayerCharacter.BP_ISOCPlayerCharacter_C"))
      (Variables|Default|SetPlayerCharacterRef (Utilities|Array|Get(acopy) _outactors_2)))
    (:then_2
      (Variables|/Game/Chameleon/Chameleon.Chameleon_C|SetRadial%20Blur (Variables|Default|GetChameleonRef) true))
    (:then_3
      (Audio|PlaySoundatLocation "/Game/AProject/Sound/SFX/132593__ceebfrack__the-portal_Cue.132593__ceebfrack__the-portal_Cue" (Transformation|GetActorLocation) "0, 0, 0" 1.0 1.0 0.0 0 0 0)
      (bind _returnvalue (Audio|SpawnSoundAttached "/Game/AProject/Sound/SFX/122972__zimbot__portal-continuous-rumble_Cue.122972__zimbot__portal-continuous-rumble_Cue" (Variables|Default|GetCapsule) "None" "0, 0, 0" "0, 0, 0" "KeepRelativeOffset" false 1.0 1.0 0.0 0 0))
      (Audio|Components|Audio|Play _returnvalue 0.0))
    (:then_4
      (bind _outactors_3 (Actor|GetAllActorsOfClass "/Game/AProject/Blueprints/BP_EndMissile.BP_EndMissile_C"))
      (Variables|Default|SetEndMissile (Utilities|Array|Get(acopy) _outactors_3)))
    (:then_5
      (bind _outactors_4 (Actor|GetAllActorsOfClass "/Script/Engine.DirectionalLight"))
      (Variables|Default|SetDirectLight (Utilities|Array|Get(acopy) _outactors_4)))
    (:then_6
      (bind _outactors_5 (Actor|GetAllActorsOfClass "/Game/AProject/Blueprints/FrameWork/BP_ISOCGameController.BP_ISOCGameController_C"))
      (Variables|Default|SetGameControllerRef (Utilities|Array|Get(acopy) _outactors_5)))
    (:then_7
      (Effects|SpawnEmitteratLocation "/Game/FXVarietyPack/Particles/P_ky_waterBallHit.P_ky_waterBallHit" (Transformation|GetActorLocation)))))

(event Collision|EventActorBeginOverlap
  (params (OtherActor :type Actor%20Object%20Reference)))

(event EventTick
  (params (DeltaSeconds :type Float%20%28single-precision%29))
  (bind _returnvalue (Transformation|GetActorLocation))
  (bind _playercharacterref (Variables|Default|GetPlayerCharacterRef))
  (bind _chameleonref (Variables|Default|GetChameleonRef))
  (bind _returnvalue_2 (Transformation|GetActorLocation _playercharacterref))
  (bind _returnvalue_3 (- _returnvalue _returnvalue_2))
  (bind _returnvalue_4 (Math|Vector|VectorLength _returnvalue_3))
  (if (< _returnvalue_4 5e+02)
    (Variables|/Game/Chameleon/Chameleon.Chameleon_C|SetRadial%20Blur%20Width _chameleonref (* (Math|Float|NormalizetoRange (* _returnvalue_4 -1.0) -5e+02 0.0) 5.0))
    (else
      (Variables|/Game/Chameleon/Chameleon.Chameleon_C|SetRadial%20Blur%20Width _chameleonref 0.0))))

(fn ConstructionScript)
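; Interactive wide door with footstep that the player triggers with the E key after entering its trigger volume.
; Trigger overlap enables input and opens a gate, so pressing E sets PlayerNear on the skeletal mesh's AnimBP_DoorWideWithFootstep.
; Leaving the trigger clears PlayerNear but neither closes the gate nor disables input.
; A failed anim instance cast draws a debug error string.
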(event OnComponentBeginOverlap(Trigger)
  (params (OverlappedComponent :type Primitive%20Component%20Object%20Reference) (OtherActor :type Actor%20Object%20Reference) (OtherComp :type Primitive%20Component%20Object%20Reference) (OtherBodyIndex :type Integer) (bFromSweep :type Boolean) (SweepResult :type Hit%20Result%20Structure%20%28by%20ref%29))
  (Input|EnableInput (Game|GetPlayerController 0))
  (Utilities|FlowControl|Gate true) ; enters at Open
)

(event OnComponentEndOverlap(Trigger)
  (params (OverlappedComponent :type Primitive%20Component%20Object%20Reference) (OtherActor :type Actor%20Object%20Reference) (OtherComp :type Primitive%20Component%20Object%20Reference) (OtherBodyIndex :type Integer))
  (bind _asanim_bp_door_wide_with_footstep (Utilities|Casting|CastToAnimBP_DoorWideWithFootstep (Components|SkeletalMesh|GetAnimInstance (Variables|Default|GetDoor_WideWithFootstep)))
    (:then
      (Variables|/Game/Interior_Toolkit_Vol_1/HQ_ResidentialHouse/Meshes/DoorWide_withFootstep/AnimBP_DoorWideWithFootstep.AnimBP_DoorWideWithFootstep_C|SetPlayerNear _asanim_bp_door_wide_with_footstep false))
    (:CastFailed
      (Rendering|Debug|DrawDebugString "0, 0, 0" "Something wrong" 0 "(R=1.000000,G=1.000000,B=1.000000,A=1.000000)" 4.0))))

(event EventBeginPlay)

(event Collision|EventActorBeginOverlap
  (params (OtherActor :type Actor%20Object%20Reference)))

(event EventTick
  (params (DeltaSeconds :type Float%20%28single-precision%29)))

(event Input|KeyboardEvents|E
  (params (Key :type Key%20Structure))
  (:Pressed
    (Utilities|FlowControl|Gate true
      (:Exit
        (bind _asanim_bp_door_wide_with_footstep (Utilities|Casting|CastToAnimBP_DoorWideWithFootstep (Components|SkeletalMesh|GetAnimInstance (Variables|Default|GetDoor_WideWithFootstep)))
          (:then
            (Variables|/Game/Interior_Toolkit_Vol_1/HQ_ResidentialHouse/Meshes/DoorWide_withFootstep/AnimBP_DoorWideWithFootstep.AnimBP_DoorWideWithFootstep_C|SetPlayerNear _asanim_bp_door_wide_with_footstep true))
          (:CastFailed
            (Rendering|Debug|DrawDebugString "0, 0, 0" "Something wrong" 0 "(R=1.000000,G=1.000000,B=1.000000,A=1.000000)" 4.0)))))))

(fn ConstructionScript)
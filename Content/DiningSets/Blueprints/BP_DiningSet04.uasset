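; BP_DiningSet04 is a dining set actor made up of a table and eight chairs that reacts to physical hits.
; On BeginPlay it binds the component hit event of every piece to one shared custom event.
; That event ignores the hit details and calls WhenHit, whose logic is defined outside this graph.
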(event Custom|커스텀%20이벤트_0
  (params (HitComponent :type Primitive%20Component%20Object%20Reference) (OtherActor :type Actor%20Object%20Reference) (OtherComp :type Primitive%20Component%20Object%20Reference) (NormalImpulse :type Vector) (Hit :type Hit%20Result%20Structure%20%28by%20ref%29))
  (CallFunction|WhenHit))

(event EventBeginPlay
  (Collision|BindEventtoOnComponentHit (Variables|Default|GetChair01) (delegate Custom|커스텀%20이벤트_0)))

(event Collision|EventActorBeginOverlap
  (params (OtherActor :type Actor%20Object%20Reference)))

(event EventTick
  (params (DeltaSeconds :type Float%20%28single-precision%29)))

(fn ConstructionScript)